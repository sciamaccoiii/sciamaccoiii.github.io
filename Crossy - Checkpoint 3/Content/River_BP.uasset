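; River_BP is a river tile actor that places an obstacle and triggers loading of the next tile as the player advances.
; Its construction script gathers five spawn-point transforms, then SpawnLogs adds a child actor component at a random one.
; When Player_BP overlaps EndTrigger, it calls LoadTile on the GM_Tutorial game mode, then destroys itself after a short delay.
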(event OnComponentBeginOverlap(EndTrigger)
  (params (OverlappedComponent :type Primitive%20Component%20Object%20Reference) (OtherActor :type Actor%20Object%20Reference) (OtherComp :type Primitive%20Component%20Object%20Reference) (OtherBodyIndex :type Integer) (bFromSweep :type Boolean) (SweepResult :type Hit%20Result%20Structure%20%28by%20ref%29))
  (Utilities|Casting|CastToPlayer_BP OtherActor)
  (bind _asgm_tutorial (Utilities|Casting|CastToGM_Tutorial (Game|GetGameMode)))
  (Default|LoadTile _asgm_tutorial)
  (Utilities|FlowControl|Delay 2.0)
  (Actor|DestroyActor))

(event EventBeginPlay
  (|CallParentFunction) ; This node is disabled and will not be called.\nDrag off pins to build functionality.
)

(event Collision|EventActorBeginOverlap
  (params (OtherActor :type Actor%20Object%20Reference))
  (|CallParentFunction OtherActor) ; This node is disabled and will not be called.\nDrag off pins to build functionality.
)

(event EventTick
  (params (DeltaSeconds :type Float%20%28single-precision%29))
  (|CallParentFunction DeltaSeconds) ; This node is disabled and will not be called.\nDrag off pins to build functionality.
)

(fn ConstructionScript
  (|CallParentFunction)
  (CallFunction|SetSpawnPoints)
  (CallFunction|SpawnLogs))

(fn SetSpawnPoints
  (Variables|Default|SetSpawnPoints (Utilities|Array|MakeArray (Transformation|GetRelativeTransform (Variables|Default|GetObstacleSpawn1)) (Transformation|GetRelativeTransform (Variables|Default|GetObstacleSpawn2)) (Transformation|GetRelativeTransform (Variables|Default|GetObstacleSpawn3)) (Transformation|GetRelativeTransform (Variables|Default|GetObstacleSpawn4)) (Transformation|GetRelativeTransform (Variables|Default|GetObstacleSpawn5)))))

(fn SpawnLogs
  (bind _spawnpoints (Variables|Default|GetSpawnPoints))
  (AddComponent|AddChildActorComponent false (Utilities|Array|Get(acopy) _spawnpoints (Math|Random|RandomIntegerinRange 0 (Utilities|Array|LastIndex _spawnpoints)))))