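; Grass tile actor for an endlessly extending level, with a randomly placed obstacle and a trigger that requests the next tile.
; The construction script caches five marker transforms in SpawnPoints, then adds a child actor component at a random one through one of two FlipFlop branches.
; When Player_BP overlaps EndTrigger, the tile calls LoadTile on GM_Tutorial and destroys itself after a short delay.
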(event OnComponentBeginOverlap(EndTrigger)
  (params (OverlappedComponent :type Primitive%20Component%20Object%20Reference) (OtherActor :type Actor%20Object%20Reference) (OtherComp :type Primitive%20Component%20Object%20Reference) (OtherBodyIndex :type Integer) (bFromSweep :type Boolean) (SweepResult :type Hit%20Result%20Structure%20%28by%20ref%29))
  (Utilities|Casting|CastToPlayer_BP OtherActor)
  (bind _asgm_tutorial (Utilities|Casting|CastToGM_Tutorial (Game|GetGameMode)))
  (Default|LoadTile _asgm_tutorial)
  (Utilities|FlowControl|Delay 2.0)
  (Actor|DestroyActor))

(event EventBeginPlay)

(event Collision|EventActorBeginOverlap
  (params (OtherActor :type Actor%20Object%20Reference)))

(event EventTick
  (params (DeltaSeconds :type Float%20%28single-precision%29)))

(fn ConstructionScript
  (CallFunction|SetSpawnPoints)
  (CallFunction|SpawnObstacles))

(fn SetSpawnPoints
  (Variables|Default|SetSpawnPoints (Utilities|Array|MakeArray (Transformation|GetRelativeTransform (Variables|Default|GetObstacleSpawn1)) (Transformation|GetRelativeTransform (Variables|Default|GetObstacleSpawn2)) (Transformation|GetRelativeTransform (Variables|Default|GetObstacleSpawn3)) (Transformation|GetRelativeTransform (Variables|Default|GetObstacleSpawn4)) (Transformation|GetRelativeTransform (Variables|Default|GetObstacleSpawn5)))))

(fn SpawnObstacles
  (bind _spawnpoints (Variables|Default|GetSpawnPoints))
  (bind _returnvalue (Utilities|Array|LastIndex _spawnpoints))
  (bind _returnvalue_2 (Math|Random|RandomIntegerinRange 0 _returnvalue))
  (bind _output (Utilities|Array|Get(acopy) _spawnpoints _returnvalue_2))
  (bind _isa (Utilities|FlowControl|FlipFlop)
    (:A
      (AddComponent|AddChildActorComponent _isa _output))
    (:B
      (AddComponent|AddChildActorComponent false _output))))