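; Road tile actor for the tutorial that requests the next tile when the player reaches its end.
; The construction script calls SpawnCar, which adds a child actor component at the SpawnPoint's relative transform.
; When Player_BP overlaps EndTrigger, it calls LoadTile on the GM_Tutorial game mode, then destroys itself after a short delay.
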(event OnComponentBeginOverlap(EndTrigger)
  (params (OverlappedComponent :type Primitive%20Component%20Object%20Reference) (OtherActor :type Actor%20Object%20Reference) (OtherComp :type Primitive%20Component%20Object%20Reference) (OtherBodyIndex :type Integer) (bFromSweep :type Boolean) (SweepResult :type Hit%20Result%20Structure%20%28by%20ref%29))
  (Utilities|Casting|CastToPlayer_BP OtherActor)
  (bind _asgm_tutorial (Utilities|Casting|CastToGM_Tutorial (Game|GetGameMode)))
  (Default|LoadTile _asgm_tutorial)
  (Utilities|FlowControl|Delay 2.0)
  (Actor|DestroyActor))

(event EventBeginPlay)

(event Collision|EventActorBeginOverlap
  (params (OtherActor :type Actor%20Object%20Reference)))

(event EventTick
  (params (DeltaSeconds :type Float%20%28single-precision%29)))

(fn ConstructionScript
  (CallFunction|SpawnCar))

(fn SpawnCar
  (AddComponent|AddChildActorComponent false (Transformation|GetRelativeTransform (Variables|Default|GetSpawnPoint))))