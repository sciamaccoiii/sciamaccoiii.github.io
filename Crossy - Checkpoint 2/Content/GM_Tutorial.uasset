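; Tutorial game mode (GM_Tutorial) that builds a path of randomly chosen lane tiles when play begins.
; BeginPlay calls LoadTile ten times, each spawning a random class from the Lanes array at NextLoadPoint.
; Each spawned tile is cast to Grass_BP, whose attach transform becomes the next load point, chaining tiles end to end.
; A failed cast leaves the load point unchanged.
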(event EventBeginPlay
  (for _index (range 0 9)
    (CallFunction|LoadTile)))

(event EventTick
  (params (DeltaSeconds :type Float%20%28single-precision%29)))

(fn ConstructionScript)

(fn LoadTile
  (bind _lanes (Variables|Default|GetLanes))
  (bind _returnvalue (Game|SpawnActorfromClass (Utilities|Array|Get(acopy) _lanes (Math|Random|RandomIntegerinRange 0 (Utilities|Array|LastIndex _lanes))) (Variables|Default|GetNextLoadPoint) "Undefined" 0 0))
  (bind _asgrass_bp (Utilities|Casting|CastToGrass_BP _returnvalue))
  (bind _attachtransform (Default|GetAttachTransform _asgrass_bp))
  (Variables|Default|SetNextLoadPoint _attachtransform))